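; BP_Hero is the player character, with Enhanced Input jump, single-axis movement along its forward vector and an orthographic camera.
; BeginPlay adds the default mapping context and takes its starting zoom from the BP_Snailcontrol actor in the level.
; Movement is ignored while the stored zoom equals that actor's zoomed-out distance.
; SetCameraZoom sets ortho width and stores the level, while SetCameraRotation sets camera roll.
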(event Input|EnhancedActionEvents|EnhancedInputActionIA_Movement
  (params (ActionValue :type Float%20%28double-precision%29) (ElapsedSeconds :type Float%20%28double-precision%29) (TriggeredSeconds :type Float%20%28double-precision%29) (InputAction :type Input%20Action%20Object%20Reference :default "/Game/Blueprints/IA_Movement.IA_Movement"))
  (if (not (== (Variables|/Game/Blueprints/BP_Snailcontrol.BP_Snailcontrol_C|GetZoomDistanceOut (stale EventBeginPlay _returnvalue)) (Variables|Default|GetZoomLevel)))
    (Pawn|Input|AddMovementInput (Transformation|GetActorForwardVector) ActionValue false)))

(event Input|EnhancedActionEvents|EnhancedInputActionIA_Jump
  (params (ActionValue :type Boolean) (ElapsedSeconds :type Float%20%28double-precision%29) (TriggeredSeconds :type Float%20%28double-precision%29) (InputAction :type Input%20Action%20Object%20Reference :default "/Game/Blueprints/IA_Jump.IA_Jump"))
  (Character|Jump))

(event EventBeginPlay
  (bind _asbp_player_controller (Utilities|Casting|CastToBP_PlayerController (Pawn|GetController)))
  (Input|AddMappingContext (PlayerController|LocalPlayerSubsystems|GetEnhancedInputLocalPlayerSubsystem _asbp_player_controller) "/Game/Blueprints/IMC_Default.IMC_Default" 0 "(bIgnoreAllPressedKeysUntilRelease=True,bForceImmediately=False,bNotifyUserSettings=False)")
  (bind _returnvalue (Actor|GetActorOfClass "/Game/Blueprints/BP_Snailcontrol.BP_Snailcontrol_C"))
  (CallFunction|SetCameraZoom (Variables|/Game/Blueprints/BP_Snailcontrol.BP_Snailcontrol_C|GetZoomDistanceIn _returnvalue)))

(event Collision|EventActorBeginOverlap
  (params (OtherActor :type Actor%20Object%20Reference)))

(event EventTick
  (params (DeltaSeconds :type Float%20%28single-precision%29)))

(fn ConstructionScript)

(fn SetCameraZoom
  (params (ZoomLevel :type Float%20%28double-precision%29))
  (Class|CameraComponent|SetOrthoWidth (Variables|Default|GetCamera) ZoomLevel)
  (Variables|Default|SetZoomLevel ZoomLevel))

(fn SetCameraRotation
  (params (xchange :type Float%20%28double-precision%29))
  (Transformation|SetRelativeTransform (Variables|Default|GetCamera) (Math|Transform|MakeTransform "0, 0, 0" (Math|Rotator|MakeRotator xchange 0.0 0.0) "1.000000,1.000000,1.000000") false false))