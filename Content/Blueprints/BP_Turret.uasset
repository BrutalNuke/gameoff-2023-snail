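; BP_Turret is a turret actor that smoothly rotates to face its current target, or back to its starting rotation when it has none.
; Each Tick it interpolates its forward vector toward the desired direction with VInterpTo, scaled by RotationSpeed.
; SetCurrentTarget only assigns the target; HasTarget is set only at BeginPlay, if a valid target already exists then.
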(event EventBeginPlay
  (Variables|Default|SetInitialRotation (Transformation|GetActorRotation))
  (Utilities|IsValid (Variables|Default|GetCurrentTarget)
    (:Is%20Valid
      (Variables|Default|SetHasTarget true))))

(event Collision|EventActorBeginOverlap
  (params (OtherActor :type Actor%20Object%20Reference)))

(event EventTick
  (params (DeltaSeconds :type Float%20%28single-precision%29))
  (if (Variables|Default|GetHasTarget)
    (Variables|Default|SetTargetDirection (- (Transformation|GetActorLocation (Variables|Default|GetCurrentTarget)) (Transformation|GetActorLocation)))
    (Variables|Default|SetTargetDirection (Math|Vector|Normalize (Variables|Default|GetTargetDirection)))
    (Transformation|SetActorRotation (Math|Conversions|RotationFromXVector (Math|Interpolation|VInterpTo (Transformation|GetActorForwardVector) (Variables|Default|GetTargetDirection) DeltaSeconds (Variables|Default|GetRotationSpeed))))
    (else
      (Transformation|SetActorRotation (Math|Conversions|RotationFromXVector (Math|Interpolation|VInterpTo (Transformation|GetActorForwardVector) (Math|Vector|GetForwardVector (Variables|Default|GetInitialRotation)) DeltaSeconds (Variables|Default|GetRotationSpeed)))))))

(fn ConstructionScript)

(fn SetCurrentTarget
  (params (Target :type Actor%20Object%20Reference))
  (Variables|Default|SetCurrentTarget Target))