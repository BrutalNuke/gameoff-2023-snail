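; Player-operated snail vehicle that moves along X, firing bullets, until its head touches a WINNING component; destruction or countdown expiry loads the death map.
; Overlapping control stations select speed, zoom or shooting, adjusted by positive/negative inputs.
; Speed and shooting share an energy pool, exposed as percentages, while a Timeline zooms the hero's camera.
; Tick moves the RenderComponent and uses Delays to throttle fire rate and the one-second countdown.
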(event OnComponentBeginOverlap(Speedup)
  (params (OverlappedComponent :type Primitive%20Component%20Object%20Reference) (OtherActor :type Actor%20Object%20Reference) (OtherComp :type Primitive%20Component%20Object%20Reference) (OtherBodyIndex :type Integer) (bFromSweep :type Boolean) (SweepResult :type Hit%20Result%20Structure%20%28by%20ref%29))
  (Variables|Default|SetCurrentAction "speed"))

(event OnComponentBeginOverlap(Lookout)
  (params (OverlappedComponent :type Primitive%20Component%20Object%20Reference) (OtherActor :type Actor%20Object%20Reference) (OtherComp :type Primitive%20Component%20Object%20Reference) (OtherBodyIndex :type Integer) (bFromSweep :type Boolean) (SweepResult :type Hit%20Result%20Structure%20%28by%20ref%29))
  (Variables|Default|SetCurrentAction "zoom"))

(event OnComponentEndOverlap(Lookout)
  (params (OverlappedComponent :type Primitive%20Component%20Object%20Reference) (OtherActor :type Actor%20Object%20Reference) (OtherComp :type Primitive%20Component%20Object%20Reference) (OtherBodyIndex :type Integer))
  (Variables|Default|SetCurrentAction ""))

(event OnComponentBeginOverlap(Shoot)
  (params (OverlappedComponent :type Primitive%20Component%20Object%20Reference) (OtherActor :type Actor%20Object%20Reference) (OtherComp :type Primitive%20Component%20Object%20Reference) (OtherBodyIndex :type Integer) (bFromSweep :type Boolean) (SweepResult :type Hit%20Result%20Structure%20%28by%20ref%29))
  (Variables|Default|SetCurrentAction "shooting"))

(event OnComponentEndOverlap(Shoot)
  (params (OverlappedComponent :type Primitive%20Component%20Object%20Reference) (OtherActor :type Actor%20Object%20Reference) (OtherComp :type Primitive%20Component%20Object%20Reference) (OtherBodyIndex :type Integer))
  (Variables|Default|SetCurrentAction ""))

(event OnComponentBeginOverlap(Head)
  (params (OverlappedComponent :type Primitive%20Component%20Object%20Reference) (OtherActor :type Actor%20Object%20Reference) (OtherComp :type Primitive%20Component%20Object%20Reference) (OtherBodyIndex :type Integer) (bFromSweep :type Boolean) (SweepResult :type Hit%20Result%20Structure%20%28by%20ref%29))
  (if (Components|ComponentHasTag OtherComp "WINNING")
    (Game|OpenLevel(byObjectReference) "/Game/Maps/Map_Won.Map_Won")))

(event OnComponentEndOverlap(Speedup)
  (params (OverlappedComponent :type Primitive%20Component%20Object%20Reference) (OtherActor :type Actor%20Object%20Reference) (OtherComp :type Primitive%20Component%20Object%20Reference) (OtherBodyIndex :type Integer))
  (Variables|Default|SetCurrentAction ""))

(event Input|EnhancedActionEvents|EnhancedInputActionIA_SnailControlPositive
  (params (ActionValue :type Boolean) (ElapsedSeconds :type Float%20%28double-precision%29) (TriggeredSeconds :type Float%20%28double-precision%29) (InputAction :type Input%20Action%20Object%20Reference :default "/Game/Blueprints/IA_SnailControlPositive.IA_SnailControlPositive"))
  (switch string (Variables|Default|GetCurrentAction)
    (:speed
      (CallFunction|SpeedIncrease))
    (:zoom
      (bind _zoomfraction (Timeline|Timeline Play)
        (:Update
          (bind _asbp_hero (Utilities|Casting|CastToBP_Hero (Game|GetPlayerCharacter 0)))
          (Default|SetCameraZoom _asbp_hero (+ (* _zoomfraction (- (Variables|Default|GetZoomDistanceOut) (Variables|Default|GetZoomDistanceIn))) (Variables|Default|GetZoomDistanceIn))))))
    (:shooting
      (CallFunction|ShootingIncrease))))

(event Input|EnhancedActionEvents|EnhancedInputActionIA_SnailControlNegative
  (params (ActionValue :type Boolean) (ElapsedSeconds :type Float%20%28double-precision%29) (TriggeredSeconds :type Float%20%28double-precision%29) (InputAction :type Input%20Action%20Object%20Reference :default "/Game/Blueprints/IA_SnailControlNegative.IA_SnailControlNegative"))
  (switch string (Variables|Default|GetCurrentAction)
    (:speed
      (CallFunction|SpeedDecrease))
    (:zoom
      (bind _zoomfraction (Timeline|Timeline Reverse)
        (:Update
          (bind _asbp_hero (Utilities|Casting|CastToBP_Hero (Game|GetPlayerCharacter 0)))
          (Default|SetCameraZoom _asbp_hero (+ (* _zoomfraction (- (Variables|Default|GetZoomDistanceOut) (Variables|Default|GetZoomDistanceIn))) (Variables|Default|GetZoomDistanceIn))))))
    (:shooting
      (CallFunction|ShootingDecrease))))

(event EventBeginPlay
  (Class|PaperTileMapComponent|SetTileMap (Variables|Default|GetSnailControlLevel) (Variables|Default|GettmBase))
  (bind _returnvalue (UserInterface|CreateWidget "/Game/Blueprints/WBP_Energy.WBP_Energy_C"))
  (UserInterface|Viewport|AddtoViewport _returnvalue 0)
  (Audio|PlaySound2D "/Game/Audio/fx/LoopingMove.LoopingMove" 1.0 1.0 0.0 0 0)
  (Audio|PlaySound2D "/Game/Audio/fx/mus-main_4m40s.mus-main_4m40s" 1.0 1.0 0.0 0 0))

(event Collision|EventActorBeginOverlap
  (params (OtherActor :type Actor%20Object%20Reference)))

(event EventTick
  (params (DeltaSeconds :type Float%20%28single-precision%29))
  (bind _shooting (Variables|Default|GetShooting))
  (Utilities|FlowControl|Sequence
    (:then_0
      (Utilities|FlowControl|Sequence
        (:then_0
          (Transformation|AddLocalOffset (Variables|Default|GetRenderComponent) (Math|Vector|MakeVector (* DeltaSeconds (Variables|Default|GetSpeed)) 0.0 0.0) false false))
        (:then_1
          (if (> _shooting 0.0)
            (Utilities|FlowControl|Delay (/ 2.0 _shooting))
            (Game|SpawnActorfromClass "/Game/Blueprints/BP_Bullet.BP_Bullet_C" (Transformation|GetWorldTransform (Variables|Default|GetScene)) "Undefined" "MultiplyWithRoot" 0 0)
            (Audio|PlaySound2D "/Game/Audio/fx/RandomLaser.RandomLaser" 1.0 1.0 0.0 0 0)))))
    (:then_1
      (Utilities|FlowControl|Delay 1.0)
      (if (== (Variables|Default|GetDisplaySeconds) 0)
        (if (== (Variables|Default|GetDisplayMinutes) 0)
          (Game|OpenLevel(byObjectReference) "/Game/Maps/Map_Died.Map_Died")
          (else
            (Variables|Default|SetDisplaySeconds 59)
            (Variables|Default|SetDisplayMinutes (- (Variables|Default|GetDisplayMinutes) 1))))
        (else
          (Variables|Default|SetDisplaySeconds (- (Variables|Default|GetDisplaySeconds) 1)))))))

(event EventDestroyed
  (Game|OpenLevel(byObjectReference) "/Game/Maps/Map_Died.Map_Died"))

(fn ConstructionScript)

(fn SpeedIncrease
  (if (> (Variables|Default|GetEnergy) 0)
    (Variables|Default|SetSpeed (+ (Variables|Default|GetSpeedChange) (Variables|Default|GetSpeed)))
    (CallFunction|EnergyDecrease)
    (CallFunction|SpeedPercentageUpdate)))

(fn SpeedDecrease
  (if (> (Variables|Default|GetSpeed) 0.0)
    (Variables|Default|SetSpeed (- (Variables|Default|GetSpeed) (Variables|Default|GetSpeedChange)))
    (CallFunction|EnergyIncrease)
    (CallFunction|SpeedPercentageUpdate)))

(fn EnergyIncrease
  (Variables|Default|SetEnergy (+ (Variables|Default|GetEnergy) 1))
  (CallFunction|EnergyPercentageUpdate))

(fn EnergyDecrease
  (Variables|Default|SetEnergy (- (Variables|Default|GetEnergy) 1))
  (CallFunction|EnergyPercentageUpdate))

(fn ShootingIncrease
  (if (> (Variables|Default|GetEnergy) 0)
    (Variables|Default|SetShooting (+ (Variables|Default|GetShooting) 1.0))
    (CallFunction|EnergyDecrease)
    (CallFunction|ShootPercentageUpdate)))

(fn ShootingDecrease
  (if (> (Variables|Default|GetShooting) 0.0)
    (Variables|Default|SetShooting (- (Variables|Default|GetShooting) 1.0))
    (CallFunction|EnergyIncrease)
    (CallFunction|ShootPercentageUpdate)))

(fn EnergyPercentageUpdate
  (Variables|Default|SetEnergyPercentage (/ (Variables|Default|GetEnergy) (Variables|Default|GetMaxEnergy))))

(fn SpeedPercentageUpdate
  (Variables|Default|SetSpeedPercentage (/ (/ (Variables|Default|GetSpeed) (Variables|Default|GetSpeedChange)) (Variables|Default|GetMaxEnergy))))

(fn ShootPercentageUpdate
  (Variables|Default|SetShootingPercentage (/ (Variables|Default|GetShooting) (Variables|Default|GetMaxEnergy))))